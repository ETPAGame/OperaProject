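; Musical score actor for a singing rhythm minigame, where the player matches a random sequence of notes.
; BeginPlay fills the score; TriggerNote draws it as spline meshes and scrolls them with a timeline paced to the rhythm.
; A looping timer compares the player's note to each entry, playing hit or miss feedback and growing or shrinking the player's sphere modifier.
; After the last note, it restores movement and triggers the player's chant.
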(event Custom|FillPartition
  (params (PartitionLength :type Integer))
  ;[1 1 1] TriggerNote
  ;;[1 1 1] Random Partition
  (for _index (range 0 PartitionLength)
    (bind _returnvalue (Utilities|Array|Add (Variables|Default|GetTableauNote) (Math|Random|RandomIntegerinRange 0 6)))
    (Development|PrintString (Utilities|String|Append "note n° " (Utilities|String|ToString(Integer) _returnvalue) " : " (Utilities|String|ToString(Integer) (Utilities|Array|Get(acopy) (Variables|Default|GetTableauNote) _returnvalue))) true true "(R=0.000000,G=0.300213,B=1.000000,A=1.000000)" 999.0)))

(event Custom|CheckNote
  ;[1 1 1] TriggerNote
  ;;[1 1 1] VerifNote
  (bind _output_get (Variables|Default|SetCounterEvent (+ (Variables|Default|GetCounterEvent) 1)))
  (if (Math|Float|NearlyEqual(Float) (Variables|/Game/Blueprints/Character/SideScrollerCharacter.SideScrollerCharacter_C|GetcurrentPlayerNote (Variables|Default|GetPlayerRef)) (Math|Conversions|ToFloat(Integer) (Utilities|Array|Get(acopy) (Variables|Default|GetTableauNote) _output_get)) 0.5)
    (CallFunction|GoodNote (Utilities|Array|Get(acopy) (Variables|Default|GetTableauNote) _output_get))
    (else
      (CallFunction|BadNote (Utilities|Array|Get(acopy) (Variables|Default|GetTableauNote) _output_get))))
  (Spline|UpdateSpline (Variables|Default|GetNote))
  (SplineMesh|UpdateMesh (Variables|Default|GetSplineMesh1))
  (if (>= (Variables|Default|GetCounterEvent) 19)
    (Utilities|Time|ClearandInvalidateTimerbyHandle (Variables|Default|GetTimerHandle))
    ;;[1 1 1] EndChant
    (CallFunction|EndChant)))

(event Custom|BadNote
  (params (BadNote :type Integer))
  (bind _playerref (Variables|Default|GetPlayerRef))
  ;[1 1 1] Feedback of hitting note
  (Rendering|SetVisibility (Variables|Default|GetNS_CircleSpline) false false)
  (Development|PrintString "Bad Note")
  (Audio|PlaySound2D (|SelctBadNote BadNote) 1.0 1.0 0.0 0 0)
  (Variables|Default|SetModifier%20Size%20Sphere%20Init (Variables|/Game/Blueprints/Character/SideScrollerCharacter.SideScrollerCharacter_C|GetModifierSizeSphere _playerref))
  (bind _newtrack_0 (Timeline|Timeline_2 PlayFromStart)
    (:Update
      (Variables|/Game/Blueprints/Character/SideScrollerCharacter.SideScrollerCharacter_C|SetModifierSizeSphere _playerref (Math|Float|Lerp (Variables|Default|GetModifier%20Size%20Sphere%20Init) (- (Variables|Default|GetModifier%20Size%20Sphere%20Init) 0.5) _newtrack_0)))))

(event Custom|GoodNote
  (params (Note :type Integer))
  (bind _playerref (Variables|Default|GetPlayerRef))
  ;[1 1 1] Feedback of hitting note
  (Rendering|SetVisibility (Variables|Default|GetNS_CircleSpline) true false)
  (Development|PrintString "GoodNote")
  (CallFunction|CamShakeLight)
  (Audio|PlaySound2D (|SelectNote Note) 1.0 1.0 0.0 0 0)
  (Variables|Default|SetModifier%20Size%20Sphere%20Init (Variables|/Game/Blueprints/Character/SideScrollerCharacter.SideScrollerCharacter_C|GetModifierSizeSphere _playerref))
  (bind _newtrack_0 (Timeline|Timeline_1 PlayFromStart)
    (:Update
      (Variables|/Game/Blueprints/Character/SideScrollerCharacter.SideScrollerCharacter_C|SetModifierSizeSphere _playerref (Math|Float|Lerp (Variables|Default|GetModifier%20Size%20Sphere%20Init) (+ (Variables|Default|GetModifier%20Size%20Sphere%20Init) 1.5) _newtrack_0)))))

(event Custom|DrawSpline
  (params (nbNote :type Integer) (Update? :type Boolean))
  (bind _note (Variables|Default|GetNote))
  ;[1 0 0.03292] Draw Spline
  (bind _result (Math|Integer|DecrementInt nbNote)
    (:%20%20
      (Utilities|FlowControl|Sequence
        (:then_0
          ;;[1 1 1] AddPoint
          (for _index (range 0 _result)
            (Class|SplineComponent|AddPoint (Variables|Default|GetNote) (Utilities|Struct|MakeSplinePoint (Math|Conversions|ToFloat(Integer) _index) (Math|Vector|MakeVector (Math|Conversions|ToFloat(Integer) (* _index 100)) 0.0 (Math|Conversions|ToFloat(Integer) (* (Utilities|Array|Get(acopy) (Variables|Default|GetTableauNote) _index) 50)))) true)))
        (:then_1
          ;;[1 1 1] Creating meshes
          (for _index_2 (range 0 (- (Spline|GetNumberOfSplinePoints (Variables|Default|GetNote)) 1))
            (bind _returnvalue (AddComponent|AddSplineMeshComponent false))
            (Utilities|Array|Add (Variables|Default|GetTabMesh) _returnvalue)
            (SplineMesh|SetStartandEnd _returnvalue (.Location (Spline|GetLocationandTangentatSplinePoint _note _index_2 "Local")) (.Tangent (Spline|GetLocationandTangentatSplinePoint _note _index_2 "Local")) (.Location (Spline|GetLocationandTangentatSplinePoint _note (+ _index_2 1) "Local")) (.Tangent (Spline|GetLocationandTangentatSplinePoint _note (+ _index_2 1) "Local")) true :!class /Script/Engine.SplineMeshComponent)))
        (:then_2
          ;;[1 1 1] Move
          (CallFunction|Move))))))

(event Custom|MovePlayerNote
  (bind _player_note (Variables|Default|Getplayer%20note))
  (bind _relativelocation (Variables|/Script/Engine.SceneComponent|GetRelativeLocation _player_note))
  ;[1 1 1] Movement
  ;;[1 1 1] MovePlayerNote
  (Transformation|SetRelativeLocation _player_note (Math|Vector|MakeVector (.x _relativelocation) (.y _relativelocation) (+ (* (Variables|/Game/Blueprints/Character/SideScrollerCharacter.SideScrollerCharacter_C|GetFloatNote (Variables|Default|GetPlayerRef)) 5e+01) (Variables|Default|GetDefaultZ))) false false))

(event Custom|move
  ;[1 1 1] Movement
  ;;[1 1 1 1 17] MoveSpline
  (Utilities|FlowControl|Delay (Variables|Default|GetDelayBeforeStart))
  (Components|Timeline|SetPlayRate (Variables|Default|GetTimeline_0) (/ 1.0 (* (Math|Conversions|ToFloat(Integer) (Utilities|Array|Length (Variables|Default|GetTableauNote))) (Variables|Default|GetRythm))))
  (bind _newtrack_0 (Timeline|Timeline_0 Play)
    (:Update
      (for _array_element (Variables|Default|GetTabMesh)
        (Transformation|SetRelativeLocation _array_element (Math|Vector|MakeVector (* _newtrack_0 1e+02 (Math|Conversions|ToFloat(Integer) (Utilities|Array|Length (Variables|Default|GetTableauNote)))) 0.0 0.0) false false)))))

(event Custom|TriggerNote
  ;[1 1 1] TriggerNote
  (Rendering|SetActorHiddenInGame false)
  (CallFunction|DrawSpline 20 false)
  (Audio|PlaySound2D "/Game/Sound/Sfx/Intro_scene.Intro_scene" 1.0 1.0 0.0 0 0)
  (bind _returnvalue (Utilities|Time|SetTimerbyEvent (delegate Custom|CheckNote) (Variables|Default|GetRythm) true (Variables|Default|GetDelayBeforeStart)))
  (Variables|Default|SetTimerHandle _returnvalue))

(event Custom|EndChant
  ;[1 1 1] TriggerNote
  ;;[1 1 1] EndChant
  (Variables|/Game/Blueprints/Character/SideScrollerCharacter.SideScrollerCharacter_C|SetCanMove? (Variables|Default|GetPlayerRef) true)
  (Default|TriggerChant (Variables|Default|GetPlayerRef)))

(event EventBeginPlay
  ;[1 1 1] BeginPlay
  (Variables|Default|SetSplineMesh (Variables|Default|GetSplineMesh1))
  (Variables|Default|SetCounterEvent -1)
  (Variables|Default|SetPlayerRef (.AsSide%20Scroller%20Character (Utilities|Casting|CastToSideScrollerCharacter (Game|GetPlayerCharacter 0))))
  (Variables|Default|SetDefaultZ (.z (Variables|/Script/Engine.SceneComponent|GetRelativeLocation (Variables|Default|Getplayer%20note))))
  (CallFunction|FillPartition 20)
  (bind _returnvalue (Actor|GetActorOfClass "/Game/Blueprints/Baron/BP_Baron.BP_Baron_C"))
  (Variables|Default|SetBaronRef _returnvalue))

(fn ConstructionScript)