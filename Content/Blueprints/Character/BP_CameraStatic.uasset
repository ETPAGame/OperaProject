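; BP_CameraStatic is a fixed side-scroller camera that becomes the view target when the player enters its trigger box.
; Entry plays a curtain change and blends the view after a short delay; a camera flagged as first starts FOV updates at BeginPlay.
; Once active, Tick smoothly interpolates FOV from the player's score.
; The first exit switches off listed spotlights and slowly resets the score; older Baron and light-retarget logic is disconnected.
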(event OnComponentBeginOverlap(Box)
  (params (OverlappedComponent :type Primitive%20Component%20Object%20Reference) (OtherActor :type Actor%20Object%20Reference) (OtherComp :type Primitive%20Component%20Object%20Reference) (OtherBodyIndex :type Integer) (bFromSweep :type Boolean) (SweepResult :type Hit%20Result%20Structure%20%28by%20ref%29))
  ;[1 1 1] Comment
  (bind _asside_scroller_character (Utilities|Casting|CastToSideScrollerCharacter OtherActor))
  ;;[1 1 1] OpenCurtains
  (Default|UpdateCurtains (Variables|/Game/Blueprints/Character/SideScrollerCharacter.SideScrollerCharacter_C|GetWidFlipBookRef _asside_scroller_character) "NewEnumerator2" true)
  (Utilities|FlowControl|Delay 0.5)
  (Game|Player|SetViewTargetwithBlend (.AsPlayer%20Controller (Utilities|Casting|CastToPlayerController (Pawn|GetController _asside_scroller_character))) self 0.6 "VTBlend_Linear" 0.0 false)
  (Variables|Default|SetMovingFOV? true))

(event OnComponentEndOverlap(Box)
  (params (OverlappedComponent :type Primitive%20Component%20Object%20Reference) (OtherActor :type Actor%20Object%20Reference) (OtherComp :type Primitive%20Component%20Object%20Reference) (OtherBodyIndex :type Integer))
  ;[0.2327 1 0] Comment
  (Utilities|Casting|CastToSideScrollerCharacter OtherActor)
  (if (not (Variables|Default|GetExited?))
    (Variables|Default|SetExited? true)
    (for _array_element (Variables|Default|GetLightToDisableAfterLeave)
      (bind _asbp_spot_light (Utilities|Casting|CastToBP_SpotLight _array_element))
      (Rendering|Components|Light|SetIntensity (Variables|/Game/Blueprints/Light/BP_SpotLight.BP_SpotLight_C|GetSpotLight _asbp_spot_light) 0.0))
    (Default|ScoreSlowReset (Variables|Default|GetRefPlayer))))

(event EventBeginPlay
  (Variables|Default|SetRefPlayer (.AsSide%20Scroller%20Character (Utilities|Casting|CastToSideScrollerCharacter (Game|GetPlayerCharacter 0))))
  (if (Variables|Default|GetIsFirst?)
    (Variables|Default|SetMovingFOV? true)))

(event EventTick
  (params (DeltaSeconds :type Float%20%28single-precision%29))
  (if (Variables|Default|GetMovingFOV?)
    (Variables|Default|SetCurrentFOV (Math|Interpolation|FInterpTo (Variables|Default|GetCurrentFOV) (Math|Float|MapRangeClamped (Variables|/Game/Blueprints/Character/SideScrollerCharacter.SideScrollerCharacter_C|GetCurrentScore (Variables|Default|GetRefPlayer)) 0.0 1.0 5e+01 71.0) (Utilities|Time|GetWorldDeltaSeconds) 1.0))
    (Camera|SetFieldOfView (Variables|CameraActor|GetCameraComponent) (Variables|Default|GetCurrentFOV))))

(fn ConstructionScript)