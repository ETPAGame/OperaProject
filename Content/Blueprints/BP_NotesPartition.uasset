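; Rhythm minigame actor for a singing "chant": builds a random note partition as a spline that the player follows with a pitch-controlled note marker.
; On trigger it generates spline meshes, scrolls them via timeline and starts the music, while Tick eases the marker toward the player's note height.
; A self-restarting CheckPoint timeline compares marker height to each spline segment, driving score, player sphere size and completion UI.
; Ending the chant restores movement, destroys the actor and shows star results.
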(event Custom|FillPartition
  (params (PartitionLength :type Integer))
  ;[1 1 1] TriggerNote
  ;;[1 1 1] Random Partition
  (for _index (range 0 PartitionLength)
    (if (not (== _index 0))
      (bind _this (CallFunction|RandomNoteA (Utilities|Array|Get(acopy) (Variables|Default|GetTableauNote) (- _index 1)) (Variables|Default|GetDeltaNote)))
      (Utilities|Array|Add (Variables|Default|GetTableauNote) _this)
      (else
        (Utilities|Array|Add (Variables|Default|GetTableauNote) (Math|Random|RandomIntegerinRange 0 6))))))

(event Custom|CheckNote
  ;[1 1 1] TriggerNote
  ;;[1 1 1] VerifNote
  (bind _output_get (Variables|Default|SetCounterEvent (+ (Variables|Default|GetCounterEvent) 1)))
  (if (Math|Float|NearlyEqual(Float) (Variables|/Game/Blueprints/Character/SideScrollerCharacter.SideScrollerCharacter_C|GetcurrentPlayerNote (Variables|Default|GetPlayerRef)) (Math|Conversions|ToFloat(Integer) (Utilities|Array|Get(acopy) (Variables|Default|GetTableauNote) _output_get)) 0.5)
    (CallFunction|GoodNote (Utilities|Array|Get(acopy) (Variables|Default|GetTableauNote) _output_get))
    (else
      (CallFunction|BadNote (Utilities|Array|Get(acopy) (Variables|Default|GetTableauNote) _output_get))))
  (Spline|UpdateSpline (Variables|Default|GetNote))
  (SplineMesh|UpdateMesh (Variables|Default|GetSplineMesh1))
  (Math|Integer|IncrementInt (Variables|Default|GetFollowingNote)
    (:%20%20
      (if (>= (Variables|Default|GetCounterEvent) 19)
        (Utilities|Time|ClearandInvalidateTimerbyHandle (Variables|Default|GetTimerHandle))
        (CallFunction|EndChant)))))

(event Custom|FlashGood
  ;[1 1 1] Make'em Flash
  (for _array_element (Variables|Default|GetLights%20Baron)
    (Default|Flashing _array_element)
    (for _array_element_2 (Variables|Default|GetLights%20Floria)
      (Default|UnFlash _array_element_2))))

(event Custom|FlashBad
  ;[1 1 1] Make'em Flash
  (for _array_element (Variables|Default|GetLights%20Floria)
    (Default|Flashing _array_element)
    (for _array_element_2 (Variables|Default|GetLights%20Baron)
      (Default|UnFlash _array_element_2))))

(event Custom|BadNote
  (params (BadNote :type Integer))
  (bind _playerref (Variables|Default|GetPlayerRef))
  ;[1 1 1] Feedback of hitting note
  (Development|PrintString "Bad Note")
  (Variables|Default|SetModifier%20Size%20Sphere%20Init (Variables|/Game/Blueprints/Character/SideScrollerCharacter.SideScrollerCharacter_C|GetModifierSizeSphere _playerref))
  (CallFunction|FlashBad)
  (bind _newtrack_0 (Timeline|Timeline_2 PlayFromStart)
    (:Update
      (Variables|/Game/Blueprints/Character/SideScrollerCharacter.SideScrollerCharacter_C|SetModifierSizeSphere _playerref (Math|Float|Lerp (Variables|Default|GetModifier%20Size%20Sphere%20Init) (- (Variables|Default|GetModifier%20Size%20Sphere%20Init) 0.5) _newtrack_0))
      (CallFunction|CheckLevelCompletion))))

(event Custom|GoodNote
  (params (Note :type Integer))
  (bind _playerref (Variables|Default|GetPlayerRef))
  ;[1 1 1] Feedback of hitting note
  (Development|PrintString "GoodNote")
  (CallFunction|CamShakeLight)
  (Variables|Default|SetModifier%20Size%20Sphere%20Init (Variables|/Game/Blueprints/Character/SideScrollerCharacter.SideScrollerCharacter_C|GetModifierSizeSphere _playerref))
  (CallFunction|FlashGood)
  (bind _newtrack_0 (Timeline|Timeline_1 PlayFromStart)
    (:Update
      (Variables|/Game/Blueprints/Character/SideScrollerCharacter.SideScrollerCharacter_C|SetModifierSizeSphere _playerref (Math|Float|Lerp (Variables|Default|GetModifier%20Size%20Sphere%20Init) (+ (Variables|Default|GetModifier%20Size%20Sphere%20Init) 1.5) _newtrack_0))
      (CallFunction|CheckLevelCompletion))))

(event Custom|DrawSpline
  (params (nbNote :type Integer) (Update? :type Boolean))
  (bind _note (Variables|Default|GetNote))
  ;[1 0 0.03292] Draw Spline
  (bind _result (Math|Integer|DecrementInt nbNote)
    (:%20%20
      (Utilities|FlowControl|Sequence
        (:then_0
          ;;[1 1 1] AddPoint
          (for _index (range 0 _result)
            (Class|SplineComponent|AddPoint (Variables|Default|GetNote) (Utilities|Struct|MakeSplinePoint (Math|Conversions|ToFloat(Integer) _index) (Math|Vector|MakeVector (Math|Conversions|ToFloat(Integer) (* _index 100)) 0.0 (Math|Conversions|ToFloat(Integer) (* (Utilities|Array|Get(acopy) (Variables|Default|GetTableauNote) _index) 50)))) false))
          (Spline|UpdateSpline (Variables|Default|GetNote)))
        (:then_1
          ;;[1 1 1] Creating meshes
          (for _index_2 (range 0 (- (Spline|GetNumberOfSplinePoints (Variables|Default|GetNote)) 1))
            (bind _returnvalue (AddComponent|AddSplineMeshComponent false))
            (Utilities|Array|Add (Variables|Default|GetTabMesh) _returnvalue)
            (SplineMesh|SetStartandEnd _returnvalue (.Location (Spline|GetLocationandTangentatSplinePoint _note _index_2 "Local")) (.Tangent (Spline|GetLocationandTangentatSplinePoint _note _index_2 "Local")) (.Location (Spline|GetLocationandTangentatSplinePoint _note (+ _index_2 1) "Local")) (.Tangent (Spline|GetLocationandTangentatSplinePoint _note (+ _index_2 1) "Local")) true :!class /Script/Engine.SplineMeshComponent)
            (AddComponent|AddStaticMeshComponent false)))
        (:then_2
          ;;[1 1 1] Move
          (CallFunction|Move))))))

(event Custom|MovePlayerNote
  (bind _player_note (Variables|Default|Getplayer%20note))
  (bind _relativelocation (Variables|/Script/Engine.SceneComponent|GetRelativeLocation _player_note))
  ;[1 1 1] Movement
  ;;[1 1 1] MovePlayerNote
  (Transformation|SetRelativeLocation _player_note (Math|Vector|MakeVector (.x _relativelocation) (.y _relativelocation) (+ (* (Variables|/Game/Blueprints/Character/SideScrollerCharacter.SideScrollerCharacter_C|GetFloatNote (Variables|Default|GetPlayerRef)) 5e+01) (Variables|Default|GetDefaultZ))) false false))

(event Custom|move
  ;[1 1 1] Movement
  ;;[1 1 1 1 17] MoveSpline
  (Utilities|FlowControl|Delay (Variables|Default|GetDelayBeforeStart))
  (Components|Timeline|SetPlayRate (Variables|Default|GetTimeline_0) (/ 1.0 (* (Math|Conversions|ToFloat(Integer) (Utilities|Array|Length (Variables|Default|GetTableauNote))) (Variables|Default|GetRythm))))
  (bind _newtrack_0 (Timeline|Timeline_0 Play)
    (:Update
      (for _array_element (Variables|Default|GetTabMesh)
        (Transformation|SetRelativeLocation _array_element (Math|Vector|MakeVector (* _newtrack_0 1e+02 (Math|Conversions|ToFloat(Integer) (Utilities|Array|Length (Variables|Default|GetTableauNote)))) 0.0 0.0) false false)))))

(event Custom|TriggerNote
  ;[1 1 1] TriggerNote
  (Rendering|SetActorHiddenInGame false)
  (CallFunction|DrawSpline 20 false)
  (bind _returnvalue (Utilities|Time|SetTimerbyEvent (delegate Custom|CheckPoint) (Variables|Default|GetRythm) false (Variables|Default|GetDelayBeforeStart)))
  (Variables|Default|SetTimerHandle _returnvalue)
  (bind _returnvalue_2 (Actor|GetActorOfClass "/Game/Blueprints/BP_TriggerNote.BP_TriggerNote_C"))
  (Default|MusicLaunch _returnvalue_2))

(event Custom|EndChant
  ;[1 1 1] TriggerNote
  ;;[1 1 1] EndChant
  (Variables|/Game/Blueprints/Character/SideScrollerCharacter.SideScrollerCharacter_C|SetCanMove? (Variables|Default|GetPlayerRef) true)
  (Default|TriggerChant (Variables|Default|GetPlayerRef) 0 false)
  (Actor|DestroyActor)
  (CallFunction|VerifEndLevel))

(event Custom|CheckPoint
  (bind _note (Variables|Default|GetNote))
  (bind _actualpoint (Variables|Default|GetActualPoint))
  (Components|Timeline|SetPlayRate (Variables|Default|GetActualCheckPoint) (/ 1.0 (Variables|Default|GetRythm)))
  (bind _newtrack_0 (Timeline|ActualCheckPoint PlayFromStart)
    (:Update
      (if (Math|Float|NearlyEqual(Float) (.z (Transformation|GetWorldLocation (Variables|Default|Getplayer%20note))) (.z (Class|SplineComponent|GetLocationatSplineInputKey _note (+ _newtrack_0 (Variables|Default|GetActualPoint)) "World")) 5e+01)
        (CallFunction|ManageScore 0.5)
        (else
          (CallFunction|ManageScore -0.5)))
      (Variables|/Game/Blueprints/Character/SideScrollerCharacter.SideScrollerCharacter_C|SetModifierSizeSphere (Variables|Default|GetPlayerRef) (Math|Float|MapRangeClamped (Variables|Default|GetCurrentScore) 0.0 4e+02 5.0 3e+01))
      (CallFunction|CheckLevelCompletion))
    (:Finished
      (Math|Integer|IncrementInt _actualpoint
        (:%20%20
          (if (< _actualpoint (Spline|GetNumberOfSplinePoints _note))
            (CallFunction|CheckPoint)
            (if (>= (Variables|Default|GetActualPoint) 19)
              (Utilities|Time|ClearandInvalidateTimerbyHandle (Variables|Default|GetTimerHandle))
              (CallFunction|EndChant))))))))

(event EventBeginPlay
  (bind _ns_notespline (Variables|Default|GetNS_NoteSpline))
  ;[1 1 1] BeginPlay
  (Variables|Default|SetSplineMesh (Variables|Default|GetSplineMesh1))
  (Variables|Default|SetCounterEvent -1)
  (Variables|Default|SetPlayerRef (.AsSide%20Scroller%20Character (Utilities|Casting|CastToSideScrollerCharacter (Game|GetPlayerCharacter 0))))
  (Variables|Default|SetDefaultZ (.z (Variables|/Script/Engine.SceneComponent|GetRelativeLocation (Variables|Default|Getplayer%20note))))
  (CallFunction|FillPartition 20)
  (bind _returnvalue (Actor|GetActorOfClass "/Game/Blueprints/Baron/BP_Baron.BP_Baron_C"))
  (Variables|Default|SetBaronRef _returnvalue)
  (Variables|Default|SetRelative%20Scale%203D (Variables|/Script/Engine.SceneComponent|GetRelativeScale3D (Variables|Default|Getplayer%20note)))
  (Niagara|SetNiagaraVariable(Float) _ns_notespline "rythme" (Variables|Default|GetRythm))
  (Niagara|SetNiagaraVariable(Float) _ns_notespline "life" (Variables|Default|GetRythm))
  (bind _outactors (Actor|GetAllActorsOfClass "/Game/Blueprints/Character/BP_CameraStatic.BP_CameraStatic_C"))
  (for _array_element _outactors
    (Variables|Default|SetLights%20Floria (Variables|/Game/Blueprints/Character/BP_CameraStatic.BP_CameraStatic_C|GetLightsFloria _array_element))
    (Variables|Default|SetLights%20Baron (Variables|/Game/Blueprints/Character/BP_CameraStatic.BP_CameraStatic_C|GetListLightToRetarget%28lightBaron%29 _array_element))))

(event EventTick
  (params (DeltaSeconds :type Float%20%28single-precision%29))
  (bind _player_note (Variables|Default|Getplayer%20note))
  (bind _relativelocation (Variables|/Script/Engine.SceneComponent|GetRelativeLocation _player_note))
  (Transformation|SetRelativeLocation _player_note (Math|Vector|MakeVector (.x _relativelocation) (.y _relativelocation) (Math|Interpolation|FInterpTo (Variables|Default|GetTempSaveNote) (+ (* (Variables|/Game/Blueprints/Character/SideScrollerCharacter.SideScrollerCharacter_C|GetFloatNote (Variables|Default|GetPlayerRef)) 1.5e+02) (Variables|Default|GetDefaultZ)) DeltaSeconds 2.0)) false false)
  (Variables|Default|SetTempSaveNote (.z _relativelocation)))

(fn ConstructionScript)

(fn PlayNote
  (params (Note :type Integer) (Rythme :type Float%20%28double-precision%29))
  (Audio|PlaySound2D 0 1.0 1.0 0.0 0 0))

(fn CheckLevelCompletion
  (Default|SetLevelCompletion (Variables|/Game/Blueprints/Character/SideScrollerCharacter.SideScrollerCharacter_C|GetWB_UI%20Ref (Variables|Default|GetPlayerRef)) (Math|Float|MapRangeClamped (Variables|Default|GetCurrentScore) 0.0 4e+02 0.0 1e+02)))

(fn VerifEndLevel
  (bind _playerref (Variables|Default|GetPlayerRef))
  (bind _wb_ui_ref (Variables|/Game/Blueprints/Character/SideScrollerCharacter.SideScrollerCharacter_C|GetWB_UI%20Ref _playerref))
  (Default|StarsbyScore _wb_ui_ref (Math|Float|MapRangeClamped (Variables|Default|GetCurrentScore) 0.0 4e+02 0.0 1e+02))
  (Default|ShowEndRes _wb_ui_ref))

(fn RandomNoteA
  (params (Before :type Integer) (Delta :type Integer))
  (bind _returnvalue (Math|Random|RandomIntegerinRange 1 Delta))
  (if (Math|Random|RandomBool)
    (return (Math|Integer|Clamp(Integer) (+ Before _returnvalue) 0 6))
    (else
      (return (Math|Integer|Clamp(Integer) (- Before _returnvalue) 0 6)))))

(fn ManageScore
  (params (Modif :type Float%20%28double-precision%29))
  (if (not (< (+ Modif (Variables|Default|GetCurrentScore)) 0.0))
    (Variables|Default|SetCurrentScore (+ Modif (Variables|Default|GetCurrentScore)))
    (else
      (Variables|Default|SetCurrentScore 0.0))))