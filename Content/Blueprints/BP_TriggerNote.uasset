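; BP_TriggerNote is a trigger volume that stops the side-scroller character and starts a chant and note sequence.
; On first box overlap it registers itself as the character's TriggerRef, disables movement, calls TriggerChant, and passes the inverse of its Loose flag to NoteLevelRef's TriggerNote.
; A DoOnce blocks repeats until RetriggerLoose sets Loose and re-arms it, so later triggers pass false.
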(event OnComponentBeginOverlap(Box)
  (params (OverlappedComponent :type Primitive%20Component%20Object%20Reference) (OtherActor :type Actor%20Object%20Reference) (OtherComp :type Primitive%20Component%20Object%20Reference) (OtherBodyIndex :type Integer) (bFromSweep :type Boolean) (SweepResult :type Hit%20Result%20Structure%20%28by%20ref%29))
  (bind _asside_scroller_character (Utilities|Casting|CastToSideScrollerCharacter OtherActor))
  (Utilities|FlowControl|DoOnce false
    (:Completed
      (Variables|/Game/Blueprints/Character/SideScrollerCharacter.SideScrollerCharacter_C|SetTriggerRef _asside_scroller_character self)
      (Variables|/Game/Blueprints/Character/SideScrollerCharacter.SideScrollerCharacter_C|SetCanMove? _asside_scroller_character false)
      (Default|TriggerChant _asside_scroller_character)
      (Default|TriggerNote (Variables|Default|GetNoteLevelRef) (not (Variables|Default|GetLoose))))))

(event Custom|RetriggerLoose
  (Variables|Default|SetLoose true)
  (Utilities|FlowControl|DoOnce false) ; enters at Reset
)

(event EventBeginPlay)

(event Collision|EventActorBeginOverlap
  (params (OtherActor :type Actor%20Object%20Reference)))

(event EventTick
  (params (DeltaSeconds :type Float%20%28single-precision%29)))

(fn ConstructionScript)