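; BP_PeopleNamed is an actor that shows a name label through a widget component and jitters a sphere vertically.
; On BeginPlay it passes its text to the WB_Name widget and stores the sphere's base location.
; A fast looping timer feeds a random Delay, after which the sphere snaps to a random height around that base.
; An unused Timeline and Lerp setup for smoother bobbing remains disconnected.
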(event Custom|Bouncy
  (Utilities|FlowControl|Delay (Math|Random|RandomFloatinRange 0.3 0.6))
  (Transformation|SetRelativeLocation (Variables|Default|GetSphere) (Math|Vector|MakeVector 0.0 0.0 (+ (Math|Random|RandomFloatinRange -7.0 7.0) (.z (Variables|Default|GetBaseLocation)))) false false))

(event EventBeginPlay
  (bind _aswb_name (Utilities|Casting|CastToWB_Name (UserInterface|GetWidget (Variables|Default|GetWidget)))
    (:then
      (Variables|/Game/Blueprints/Widget/WB_Name.WB_Name_C|SetTextUI _aswb_name (Variables|Default|GetTextWid)))
    (:CastFailed
      _))
  (Variables|Default|SetBaseLocation (Variables|/Script/Engine.SceneComponent|GetRelativeLocation (Variables|Default|GetSphere)))
  (Utilities|Time|SetTimerbyEvent (delegate Custom|Bouncy) 0.1 true))

(fn ConstructionScript)