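; Singing-minigame note track that turns a note array into a scrolling melody the player must match by pitch.
; TriggerNote reveals it and builds a spline with spline meshes from the array.
; The move event plays sound, then a rhythm-scaled timeline scrolls the track, raising score and toggling success Niagara while pitches align.
; Tick eases the player marker toward the character's FloatNote; on finish, it ends singing and destroys itself.
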(event Custom|move
  (bind _playerref (Variables|Default|GetPlayerRef))
  ;[1 1 1] Movement
  (Variables|Default|SetMoving true)
  (Audio|PlaySound2D (Variables|Default|GetSoundsToplay) 1.0 1.0 0.0 0 0)
  (Utilities|FlowControl|Delay (Variables|Default|GetDelayBeforeStart))
  (Variables|Default|SetTimelineSpeed (/ 1.0 (* (Utilities|Array|Length (Variables|Default|GetTableauNote)) (Variables|Default|GetRythm))))
  (Components|Timeline|SetPlayRate (Variables|Default|GetMovement) (Variables|Default|GetTimelineSpeed))
  (bind _musiclength (Timeline|Movement PlayFromStart)
    (:Update
      (Utilities|FlowControl|Sequence
        (:then_0
          (for _array_element (Variables|Default|GetTabMesh)
            (Transformation|SetRelativeLocation _array_element (Math|Vector|MakeVector (* (* _musiclength (Utilities|Array|LastIndex (Variables|Default|GetTableauNote))) -1e+02) 0.0 0.0) false false)))
        (:then_1
          (Transformation|SetRelativeLocation (Variables|Default|GetNote) (Math|Vector|MakeVector (* (* _musiclength (Utilities|Array|LastIndex (Variables|Default|GetTableauNote))) -1e+02) 0.0 0.0) false false))
        (:then_2
          (CallFunction|ManageScore (select (Math|Float|NearlyEqual(Float) (.z (Class|SplineComponent|GetLocationatSplineInputKey (Variables|Default|GetNote) (* _musiclength (Utilities|Array|LastIndex (Variables|Default|GetTableauNote))) "World")) (.z (Transformation|GetWorldLocation (Variables|Default|Getplayer%20note))) 5e+01) (* (Variables|Default|GetTimelineSpeed) (Utilities|Time|GetWorldDeltaSeconds)) 0.0))
          (if (Math|Float|NearlyEqual(Float) (.z (Class|SplineComponent|GetLocationatSplineInputKey (Variables|Default|GetNote) (* _musiclength (Utilities|Array|LastIndex (Variables|Default|GetTableauNote))) "World")) (.z (Transformation|GetWorldLocation (Variables|Default|Getplayer%20note))) 5e+01)
            (Utilities|FlowControl|DoOnce false :!label _label
              (:Completed
                (Components|Activation|Activate (Variables|Default|GetNS_SuccessSpline) false)
                (goto _label_2 Reset)))
            (else
              (Utilities|FlowControl|DoOnce false :!label _label_2
                (:Completed
                  (Components|Activation|Deactivate (Variables|Default|GetNS_SuccessSpline))
                  (goto _label Reset))))))
        (:then_3
          (Default|SetLevelCompletion (Variables|/Game/Blueprints/Character/SideScrollerCharacter.SideScrollerCharacter_C|GetWB_UI%20Ref _playerref) (Variables|/Game/Blueprints/Character/SideScrollerCharacter.SideScrollerCharacter_C|GetCurrentScore _playerref)))))
    (:Finished
      (Default|EndSing (Variables|Default|GetPlayerRef))
      (Actor|DestroyActor))))

(event Custom|TriggerNote
  (Rendering|SetActorHiddenInGame false)
  (CallFunction|DrawSplineFunct))

(event EventBeginPlay
  (bind _ns_notespline (Variables|Default|GetNS_NoteSpline))
  ;[1 1 1] BeginPlay
  (Variables|Default|SetPlayerRef (.AsSide%20Scroller%20Character (Utilities|Casting|CastToSideScrollerCharacter (Game|GetPlayerCharacter 0))))
  (Variables|Default|SetDefaultZ (.z (Variables|/Script/Engine.SceneComponent|GetRelativeLocation (Variables|Default|Getplayer%20note))))
  (Niagara|SetNiagaraVariable(Float) _ns_notespline "rythme" (Variables|Default|GetRythm))
  (Niagara|SetNiagaraVariable(Float) _ns_notespline "life" (Variables|Default|GetRythm)))

(event EventTick
  (params (DeltaSeconds :type Float%20%28single-precision%29))
  (bind _player_note (Variables|Default|Getplayer%20note))
  (bind _relativelocation (Variables|/Script/Engine.SceneComponent|GetRelativeLocation _player_note))
  (Transformation|SetRelativeLocation _player_note (Math|Vector|MakeVector (.x _relativelocation) (.y _relativelocation) (Math|Interpolation|FInterpTo (Variables|Default|GetTempSaveNote) (+ (* (Variables|/Game/Blueprints/Character/SideScrollerCharacter.SideScrollerCharacter_C|GetFloatNote (Variables|Default|GetPlayerRef)) 1.5e+02) (Variables|Default|GetDefaultZ)) (Utilities|Time|GetWorldDeltaSeconds) 2.0)) false false)
  (Variables|Default|SetTempSaveNote (.z _relativelocation)))

(fn ConstructionScript)

(fn ManageScore
  (params (Modif :type Float%20%28double-precision%29))
  (Variables|/Game/Blueprints/Character/SideScrollerCharacter.SideScrollerCharacter_C|SetCurrentScore (Variables|Default|GetPlayerRef) (Math|Float|Clamp(Float) (select (< (+ Modif (Variables|/Game/Blueprints/Character/SideScrollerCharacter.SideScrollerCharacter_C|GetCurrentScore (Variables|Default|GetPlayerRef))) 0.0) 0.0 (+ Modif (Variables|/Game/Blueprints/Character/SideScrollerCharacter.SideScrollerCharacter_C|GetCurrentScore (Variables|Default|GetPlayerRef)))))))

(fn DrawSplineFunct
  (bind _note (Variables|Default|GetNote))
  ;[1 0 0.03292] Draw Spline
  (Utilities|FlowControl|Sequence
    (:then_0
      ;;[1 1 1] AddPoint
      (for (_array_element _array_index) (Variables|Default|GetTableauNote)
        (if (== _array_index 0)
          (Spline|SetLocationatSplinePoint (Variables|Default|GetNote) 0 (Math|Vector|MakeVector (Math|Conversions|ToFloat(Integer) (* _array_index 100)) 0.0 (Math|Conversions|ToFloat(Integer) (* _array_element 50))) "Local" false)
          (else
            (Class|SplineComponent|AddPoint (Variables|Default|GetNote) (Utilities|Struct|MakeSplinePoint (Math|Conversions|ToFloat(Integer) _array_index) (Math|Vector|MakeVector (Math|Conversions|ToFloat(Integer) (* _array_index 100)) 0.0 (Math|Conversions|ToFloat(Integer) (* _array_element 50)))) false))))
      (Spline|UpdateSpline (Variables|Default|GetNote)))
    (:then_1
      ;;[1 1 1] Creating meshes
      (for _index (range 0 (- (Utilities|Array|LastIndex (Variables|Default|GetTableauNote)) 1))
        (bind _returnvalue (AddComponent|AddSplineMeshComponent false))
        (Utilities|Array|Add (Variables|Default|GetTabMesh) _returnvalue)
        (SplineMesh|SetStartandEnd _returnvalue (.Location (Spline|GetLocationandTangentatSplinePoint _note _index "Local")) (.Tangent (Spline|GetLocationandTangentatSplinePoint _note _index "Local")) (.Location (Spline|GetLocationandTangentatSplinePoint _note (+ _index 1) "Local")) (.Tangent (Spline|GetLocationandTangentatSplinePoint _note (+ _index 1) "Local")) true :!class /Script/Engine.SplineMeshComponent)))))