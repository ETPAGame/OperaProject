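; Links the player's movement speed to a Kuwahara post-process filter, so the effect strengthens as the player moves faster.
; On BeginPlay it creates a dynamic instance of PPI_Kuwahara and replaces the referenced post-process settings with it as a blendable.
; A quarter-speed timeline then updates the X and Y radii identically, multiplying its curve by a non-linear factor of clamped player speed.
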(event EventBeginPlay
  (bind _playerref (Variables|Default|GetPlayerRef))
  (bind _returnvalue (Transformation|GetVelocity _playerref))
  (bind _returnvalue_2 (Math|Vector|VectorLength _returnvalue))
  (bind _returnvalue_3 (Math|Float|MapRangeClamped _returnvalue_2 0.0 6e+02 0.0 1.0))
  (bind _returnvalue_4 (Rendering|Material|CreateDynamicMaterialInstance "/Game/PaintFilter/Materials/PostProcess/PPI_Kuwahara.PPI_Kuwahara" "None" "None" :!class /Script/Engine.KismetMaterialLibrary))
  (Variables|Default|SetMat _returnvalue_4)
  (Variables|/Script/Engine.PostProcessVolume|SetSettings (Variables|Default|GetPostProcessRef) (Utilities|Struct|MakePostProcessSettings (Utilities|Struct|MakeWeightedBlendables (Utilities|Array|MakeArray (Utilities|Struct|MakeWeightedBlendable 1.0 (Variables|Default|GetMat))))))
  (Components|Timeline|SetPlayRate (Variables|Default|GetVariationPostProcess) 0.25)
  (bind _newtrack_0 (Timeline|VariationPostProcess Play)
    (:Update
      (Rendering|Material|SetScalarParameterValue (Variables|Default|GetMat) "XRadius" (* _returnvalue_3 _newtrack_0 (+ _returnvalue_3 2.0) 5.0) :!class /Script/Engine.MaterialInstanceDynamic)
      (Rendering|Material|SetScalarParameterValue (Variables|Default|GetMat) "YRadius" (* _returnvalue_3 _newtrack_0 (+ _returnvalue_3 2.0) 5.0) :!class /Script/Engine.MaterialInstanceDynamic))))

(fn ConstructionScript)