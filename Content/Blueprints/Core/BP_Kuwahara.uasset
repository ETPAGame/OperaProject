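; BP_Kuwahara is a post-process actor that applies a Kuwahara filter effect whose radius grows with the player's movement speed.
; The construction script creates a dynamic instance of PPI_Kuwahara and, when Activate is set, adds it to the PostProcess component as a low-weight blendable.
; Each tick it maps the SideScrollerCharacter's speed to a radius, smooths it with FInterpTo, and drives both XRadius and YRadius.
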(event EventBeginPlay
  (Variables|Default|SetPlayerRef (.AsSide%20Scroller%20Character (Utilities|Casting|CastToSideScrollerCharacter (Game|GetPlayerCharacter 0)))))

(event EventTick
  (params (DeltaSeconds :type Float%20%28single-precision%29))
  (bind _mat (Variables|Default|GetMat)
    (:then
      (Rendering|Material|SetScalarParameterValue _mat "XRadius" (Math|Interpolation|FInterpTo (Variables|Default|GetCurrentValue) (Math|Float|MapRangeClamped (Math|Vector|VectorLength (Transformation|GetVelocity (Variables|Default|GetPlayerRef))) 0.0 6e+02 4.0 1e+01) DeltaSeconds 1e+01) :!class /Script/Engine.MaterialInstanceDynamic)
      (Rendering|Material|SetScalarParameterValue _mat "YRadius" (Math|Interpolation|FInterpTo (Variables|Default|GetCurrentValue) (Math|Float|MapRangeClamped (Math|Vector|VectorLength (Transformation|GetVelocity (Variables|Default|GetPlayerRef))) 0.0 6e+02 4.0 1e+01) DeltaSeconds 1e+01) :!class /Script/Engine.MaterialInstanceDynamic)
      (Variables|Default|SetCurrentValue (Math|Interpolation|FInterpTo (Variables|Default|GetCurrentValue) (Math|Float|MapRangeClamped (Math|Vector|VectorLength (Transformation|GetVelocity (Variables|Default|GetPlayerRef))) 0.0 6e+02 4.0 1e+01) DeltaSeconds 1e+01)))
    (:else)))

(fn ConstructionScript
  (Utilities|FlowControl|Sequence
    (:then_0
      (Variables|Default|GetMat
        (:then)
        (:else
          (bind _returnvalue (Rendering|Material|CreateDynamicMaterialInstance "/Game/Materials/PostProcess/PPI_Kuwahara.PPI_Kuwahara" "None" "None" :!class /Script/Engine.KismetMaterialLibrary))
          (Variables|Default|SetMat _returnvalue))))
    (:then_1
      (if (Variables|Default|GetActivate)
        (Variables|/Script/Engine.PostProcessComponent|SetSettings (Variables|Default|GetPostProcess) (Utilities|Struct|MakePostProcessSettings (Utilities|Struct|MakeWeightedBlendables (Utilities|Array|MakeArray (Utilities|Struct|MakeWeightedBlendable 0.15 (Variables|Default|GetMat))))))))))