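; BP_Baron is an actor that flees and disappears when the side-scroller player character enters its trigger box.
; The box overlap ignores static mesh and Niagara components, then plays the AM_Fuite montage and destroys the actor on completion.
; An unconnected timeline holds multi-position flee logic that turns and moves the capsule through ArrayFleePos by CurrentScene.
; The chant event is an empty stub.
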(event OnComponentBeginOverlap(Box)
  (params (OverlappedComponent :type Primitive%20Component%20Object%20Reference) (OtherActor :type Actor%20Object%20Reference) (OtherComp :type Primitive%20Component%20Object%20Reference) (OtherBodyIndex :type Integer) (bFromSweep :type Boolean) (SweepResult :type Hit%20Result%20Structure%20%28by%20ref%29))
  (Utilities|Casting|CastToStaticMeshComponent OtherComp
    (:CastFailed
      (Utilities|Casting|CastToNiagaraComponent OtherComp
        (:CastFailed
          (Utilities|Casting|CastToSideScrollerCharacter OtherActor)
          (Animation|Montage|PlayMontage (Variables|Character|GetMesh) "/Game/Characters/Baron/Animations/AM_Fuite.AM_Fuite"
            (:OnCompleted
              (Actor|DestroyActor))))))))

(event Custom|chant)

(fn ConstructionScript)